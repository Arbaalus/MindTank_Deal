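; BP_BaseVehicle is a base Chaos wheeled vehicle Blueprint providing wheel effects and engine audio.
; Each Tick spawns emitters at the first three wheels' contact points above a speed threshold; surface-type selection is unconnected.
; It also maps engine RPM to a sound parameter, muting audio when the engine is off.
; GetPawnAnimBP passes the vehicle type to a character's Synty AnimBP; BikeToAnimBpPawn is empty.
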(event `self.ReceiveBeginPlay`
  (bind _aschaos_wheeled_vehicle_movement_component (cast `ChaosWheeledVehicleMovementComponent` (`self.VehicleMovementComponent`)))
  (set `self.Wheels Component` _aschaos_wheeled_vehicle_movement_component))

(event `self.ReceiveTick`
  (params (DeltaSeconds :type "Float (single-precision)"))
  (`self.SurfaceEffect`)
  (`self.EngineSoundsRPM`))

(fn `BikeToAnimBpPawn`)

(fn `EngineSoundsRPM`
  (bind _wheels_component (`self.Wheels Component`))
  (bind _enginesound (`self.EngineSound`))
  (`/Engine/EditorBlueprintResources/StandardMacros.IsValid` _wheels_component
    (:`Is Valid`
      (if (`self.EngineOn`)
        (`AudioComponent.SetVolumeMultiplier` _enginesound 1.0)
        (`AudioComponent.SetFloatParameter` _enginesound "RPM" (`KismetMathLibrary.MapRangeClamped` (`ChaosWheeledVehicleMovementComponent.GetEngineRotationSpeed` _wheels_component) 1200.0 (`ChaosWheeledVehicleMovementComponent.GetEngineMaxRotationSpeed` _wheels_component) 0.0 1.0))
        (else
          (`AudioComponent.SetVolumeMultiplier` _enginesound 0.0))))))

(fn `GetPawnAnimBP`
  (params (Character :type "/Game/MurratProj/Blueprint/Character_BP/BP_Charac_Player_FinalB Object Reference"))
  (bind _assynty_anim_bp (cast `/Game/MurratProj/Animation/AnimBp/Synty_AnimBP` (`SkeletalMeshComponent.GetAnimInstance` (`Character.Mesh` Character))))
  (bind _output_get (set `self.Anim BP` _assynty_anim_bp))
  (set `/Game/MurratProj/Animation/AnimBp/Synty_AnimBP.Vehicle` (`self.VehicleType`) _output_get))

(fn `SurfaceEffect`
  (bind _wheels_component (`self.Wheels Component`))
  (`/Engine/EditorBlueprintResources/StandardMacros.IsValid` _wheels_component
    (:`Is Valid`
      (bind (_bincontact _contactpoint _physmaterial) (`ChaosWheeledVehicleMovementComponent.BreakWheelStatus` (`ChaosWheeledVehicleMovementComponent.GetWheelState` _wheels_component (stale _array_index))))
      (if (and (> (`KismetMathLibrary.VSize` (`self.GetVelocity`)) 400.0) _bincontact)
        (for (_ _array_index) (`ChaosWheeledVehicleMovementComponent.Wheels` _wheels_component)
          (if (< _array_index 3)
            (`/Engine/EditorBlueprintResources/StandardMacros.IsValid` _physmaterial
              (:`Is Valid`
                (`GameplayStatics.SpawnEmitterAtLocation` null _contactpoint)))))))))

(fn `UserConstructionScript`)
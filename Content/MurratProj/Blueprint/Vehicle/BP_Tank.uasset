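; Player-drivable tank vehicle that steers by physics torque, turns its turret and fires shell projectiles.
; Steering adds yaw torque while angular velocity stays within limits; throttle is left to the parent class.
; Tick accumulates look input into turret yaw and scrolls two dynamic track materials by movement and steering direction.
; Firing spawns a shell at ShootDir with a world camera shake; turret pitch logic is unconnected.
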(event `self.ReceiveBeginPlay`
  (bind _mesh (`self.Mesh`))
  (`parent.ReceiveBeginPlay`)
  (bind _returnvalue (`PrimitiveComponent.CreateDynamicMaterialInstance` _mesh 1 "/Game/Polygon_BattleRoyale/Materials/Mat_PolygonBattleRoyale_TankTracks_L.Mat_PolygonBattleRoyale_TankTracks_L" "None"))
  (set `self.TrackL` _returnvalue)
  (bind _returnvalue_2 (`PrimitiveComponent.CreateDynamicMaterialInstance` _mesh 2 "/Game/Polygon_BattleRoyale/Materials/Mat_PolygonBattleRoyale_TankTracks_L.Mat_PolygonBattleRoyale_TankTracks_L" "None"))
  (set `self.TrackR` _returnvalue_2))

(event `self.ReceiveTick`
  (params (DeltaSeconds :type "Float (single-precision)"))
  (bind (_returnvalue_x _returnvalue_y) (`KismetMathLibrary.BreakVector2D` (`|GetInputActionValue`)))
  (`parent.ReceiveTick` DeltaSeconds)
  (`self.TrackThrottle`)
  (set `self.TurretTurn` (+ _returnvalue_x (`self.TurretTurn`))))

(event `EnhancedInput|/Game/MurratProj/Blueprint/Vehicle/VehicleInput/TankFire`
  (params (ActionValue :type Boolean) (ElapsedSeconds :type "Float (double-precision)") (TriggeredSeconds :type "Float (double-precision)") (InputAction :type "InputAction Object Reference" :default "/Game/MurratProj/Blueprint/Vehicle/VehicleInput/TankFire.TankFire"))
  (:`Started`
    (`self.Fire`)
    (`GameplayStatics.PlayWorldCameraShake` "/Game/MurratProj/Blueprint/Vehicle/BP_TankCamShake.BP_TankCamShake_C" (`self.K2_GetActorLocation`) 1000.0 1500.0 1.0 true)))

(fn `Fire`
  (`|SpawnActorFromClass` "/Game/MurratProj/Blueprint/Weapons/Gun/Projectile/BP_Projectile_TankObus.BP_Projectile_TankObus_C" (`SceneComponent.K2_GetComponentToWorld` (`self.ShootDir`)) "Undefined" "MultiplyWithRoot" null null))

(fn `Set Track Speed`
  (params (TrackL :type "Float (single-precision)") (TrackR :type "Float (single-precision)"))
  (`MaterialInstanceDynamic.SetVectorParameterValue` (`self.TrackL`) "TrackSpeed" (make `LinearColor` 0.0 TrackL))
  (`MaterialInstanceDynamic.SetVectorParameterValue` (`self.TrackR`) "TrackSpeed" (make `LinearColor` 0.0 TrackR)))

(fn `SetSteering`
  (params (Steering :type "Float (single-precision)"))
  (bind _returnvalue (* Steering 500.0))
  (bind (_returnvalue_x _returnvalue_y _returnvalue_z) (`KismetMathLibrary.BreakVector` (`PrimitiveComponent.GetPhysicsAngularVelocityInDegrees` (`self.Mesh`) "None")))
  (set `self.Steering` Steering)
  (set `self.ActTorque` _returnvalue)
  (if (`KismetMathLibrary.InRange_FloatFloat` _returnvalue_z -100.0 100.0)
    (`PrimitiveComponent.AddTorqueInDegrees` (`self.Mesh`) (`KismetMathLibrary.MakeVector` 0.0 0.0 _returnvalue) "None" true)))

(fn `SetThrottle`
  (params (Throttle :type "Float (single-precision)"))
  (`parent.SetThrottle` Throttle))

(fn `TrackThrottle`
  (bind _steering (`self.Steering`))
  (if (or (> (`KismetMathLibrary.VSize` (`self.GetVelocity`)) 50.0) (!= (`self.Steering`) 0.0))
    (`self.Set Track Speed` (`KismetMathLibrary.SelectFloat` 2.0 -2.0 (< _steering 0.0)) (`KismetMathLibrary.SelectFloat` 2.0 -2.0 (> _steering 0.0)))
    (else
      (`self.Set Track Speed` 0.0))))

(fn `UserConstructionScript`
  (`parent.UserConstructionScript`))
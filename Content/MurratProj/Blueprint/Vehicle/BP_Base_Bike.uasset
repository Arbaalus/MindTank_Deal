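; BP_Base_Bike is the base Blueprint for bike vehicles, extending a parent vehicle class to drive the rider's animation.
; While a driver is present, each tick writes lean and speed to the AnimBP reference.
; Lean is the bike's roll remapped to a clamped normalized range, and speed is the raw velocity magnitude.
; Construction, anim Blueprint lookup and possess effects only call the parent, leaving some unconnected leftover nodes.
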(event `self.ReceiveTick`
  (params (DeltaSeconds :type "Float (single-precision)"))
  (`parent.ReceiveTick` DeltaSeconds)
  (if (`self.HasDriver`)
    (`self.BikeToAnimBpPawn`)))

(fn `BikeToAnimBpPawn`
  (bind _returnvalue_roll (`KismetMathLibrary.BreakRotator` (`self.K2_GetActorRotation`)))
  (bind _anim_bp (`self.Anim BP`)
    (:`then`
      (set `/Game/MurratProj/Animation/AnimBp/Synty_AnimBP.Lean` (`KismetMathLibrary.MapRangeClamped` _returnvalue_roll -40.0 40.0 -1.0 1.0) _anim_bp)
      (set `/Game/MurratProj/Animation/AnimBp/Synty_AnimBP.VehicleSpeed` (`KismetMathLibrary.VSize` (`self.GetVelocity`)) _anim_bp))
    (:`else`)))

(fn `GetPawnAnimBP`
  (params (Character :type "/Game/MurratProj/Blueprint/Character_BP/BP_Charac_Player_FinalB Object Reference"))
  (`parent.GetPawnAnimBP` Character))

(fn `PossessEffect`
  (`parent.PossessEffect`))

(fn `UserConstructionScript`
  (`parent.UserConstructionScript`))
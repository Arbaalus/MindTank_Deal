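; Player-flown helicopter pawn (named as an old version) that disables gravity and moves kinematically through Enhanced Input.
; Input handlers ease pitch, yaw, roll and lift speeds with FInterpTo, banking into turns and self-leveling without input.
; Tick applies local offset and rotation, derives forward speed from pitch, and swings control yaw toward the heading when moving forward.
; The engine and blade-speed check is unconnected.
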(event `self.ReceiveBeginPlay`
  (bind _asplayer_controller (cast `PlayerController` (`self.GetController`)))
  (bind _returnvalue (pcsubsystem `EnhancedInputLocalPlayerSubsystem` _asplayer_controller))
  (`/Engine/EditorBlueprintResources/StandardMacros.IsValid` _returnvalue
    (:`Is Valid`
      (`EnhancedInputSubsystemInterface.AddMappingContext` _returnvalue "/Game/MurratProj/Blueprint/Vehicle/VehicleInput/IMC_Chopper.IMC_Chopper" 0 (struct))
      (`PrimitiveComponent.SetEnableGravity` (`self.SK_Veh_Helicopter_01`) false))))

(event `EnhancedInput|/Game/MurratProj/Blueprint/Vehicle/VehicleInput/YawTurnR`
  (params (ActionValue :type Boolean) (ElapsedSeconds :type "Float (double-precision)") (TriggeredSeconds :type "Float (double-precision)") (InputAction :type "InputAction Object Reference" :default "/Game/MurratProj/Blueprint/Vehicle/VehicleInput/YawTurnR.YawTurnR"))
  (:`Started`
    (set `self.ShoulderYaw` 20.0)
    (set `self.CurrentYawSpeed` (`KismetMathLibrary.FInterpTo` (`self.CurrentYawSpeed`) (* (`self.ShoulderYaw`) (`self.TurnSpeed`)) (`GameplayStatics.GetWorldDeltaSeconds`) 2.0) :!label _label)))

(event `EnhancedInput|/Game/MurratProj/Blueprint/Vehicle/VehicleInput/YawTurnL`
  (params (ActionValue :type Boolean) (ElapsedSeconds :type "Float (double-precision)") (TriggeredSeconds :type "Float (double-precision)") (InputAction :type "InputAction Object Reference" :default "/Game/MurratProj/Blueprint/Vehicle/VehicleInput/YawTurnL.YawTurnL"))
  (:`Started`
    (set `self.ShoulderYaw` -20.0)
    (goto _label)))

(event `EnhancedInput|/Game/MurratProj/Blueprint/Vehicle/VehicleInput/ThrottleUp`
  (params (ActionValue :type "Float (double-precision)") (ElapsedSeconds :type "Float (double-precision)") (TriggeredSeconds :type "Float (double-precision)") (InputAction :type "InputAction Object Reference" :default "/Game/MurratProj/Blueprint/Vehicle/VehicleInput/ThrottleUp.ThrottleUp"))
  (:`Triggered`
    (`self.VerticalMove` ActionValue (stale `EnhancedInput|/Game/MurratProj/Blueprint/Vehicle/VehicleInput/ThrottleDown` ActionValue) :!label _label_2))
  (:`Completed`
    (goto _label_2)))

(event `EnhancedInput|/Game/MurratProj/Blueprint/Vehicle/VehicleInput/ChopperForward`
  (params (ActionValue :type "Float (double-precision)") (ElapsedSeconds :type "Float (double-precision)") (TriggeredSeconds :type "Float (double-precision)") (InputAction :type "InputAction Object Reference" :default "/Game/MurratProj/Blueprint/Vehicle/VehicleInput/ChopperForward.ChopperForward"))
  (:`Triggered`
    (`self.ForwardMove` ActionValue :!label _label_3))
  (:`Completed`
    (goto _label_3)))

(event `EnhancedInput|/Game/MurratProj/Blueprint/Vehicle/VehicleInput/ThrottleDown`
  (params (ActionValue :type "Float (double-precision)") (ElapsedSeconds :type "Float (double-precision)") (TriggeredSeconds :type "Float (double-precision)") (InputAction :type "InputAction Object Reference" :default "/Game/MurratProj/Blueprint/Vehicle/VehicleInput/ThrottleDown.ThrottleDown"))
  (:`Triggered`
    (goto _label_2))
  (:`Completed`
    (goto _label_2)))

(event `EnhancedInput|/Game/MurratProj/Blueprint/Vehicle/VehicleInput/Steering`
  (params (ActionValue :type "Float (double-precision)") (ElapsedSeconds :type "Float (double-precision)") (TriggeredSeconds :type "Float (double-precision)") (InputAction :type "InputAction Object Reference" :default "/Game/MurratProj/Blueprint/Vehicle/VehicleInput/Steering.Steering"))
  (:`Triggered`
    (`self.TurnMove` ActionValue :!label _label_4))
  (:`Completed`
    (goto _label_4)))

(event `self.ReceiveTick`
  (params (DeltaSeconds :type "Float (single-precision)"))
  (`|ExecutionSequence`
    (:`then_0`
      (`self.UppdateLocalOffset` DeltaSeconds))
    (:`then_1`
      (`self.UppdateRotation`)
      (`self.SetForwardSpeed`))
    (:`then_2`
      (`self.UppdateControllerYaw`))))

(fn `ForwardMove`
  (params (AxisValue :type "Float (double-precision)"))
  (set `self.CurentPitchSpeed` (`KismetMathLibrary.FInterpTo` (`self.CurentPitchSpeed`) (`KismetMathLibrary.SelectFloat` (* (* AxisValue -1.0) (`self.TurnSpeed`)) (* (.pitch (`self.K2_GetActorRotation`)) -0.5) (and (> (`KismetMathLibrary.Abs` AxisValue) 0.0) (`KismetMathLibrary.InRange_FloatFloat` (.pitch (`self.K2_GetActorRotation`)) -50.0 50.0 false false))) (`GameplayStatics.GetWorldDeltaSeconds`) 2.0)))

(fn `SetForwardSpeed`
  (bind _currentforwardspeed (`self.CurrentForwardSpeed`))
  (bind _pitch (.pitch (`self.K2_GetActorRotation`)))
  (`/Engine/EditorBlueprintResources/StandardMacros.CompareFloat` _pitch -5.0
    (:`>`
      (`/Engine/EditorBlueprintResources/StandardMacros.CompareFloat` _pitch 5.0
        (:`>`
          (`/Engine/EditorBlueprintResources/StandardMacros.CompareFloat` _currentforwardspeed -500.0
            (:`>`
              (set `self.CurrentForwardSpeed` (- _currentforwardspeed 10.0)))))
        (:`==`
          (set `self.CurrentForwardSpeed` (`KismetMathLibrary.FInterpTo` _currentforwardspeed 0.0 (`GameplayStatics.GetWorldDeltaSeconds`) 0.5) :!label _label))
        (:`<`
          (goto _label))))
    (:`<`
      (`/Engine/EditorBlueprintResources/StandardMacros.CompareFloat` _currentforwardspeed 2500.0
        (:`<`
          (set `self.CurrentForwardSpeed` (+ _currentforwardspeed 10.0)))))))

(fn `TurnMove`
  (params (AxisValue :type "Float (double-precision)"))
  (set `self.CurrentYawSpeed` (`KismetMathLibrary.FInterpTo` (`self.CurrentYawSpeed`) (* AxisValue (`self.TurnSpeed`)) (`GameplayStatics.GetWorldDeltaSeconds`) 2.0))
  (set `self.CurrentRollSpeed` (`KismetMathLibrary.FInterpTo` (`self.CurrentRollSpeed`) (`KismetMathLibrary.SelectFloat` (* (`self.CurrentYawSpeed`) 0.8) (* (.roll (`self.K2_GetActorRotation`)) -2.0) (> (`KismetMathLibrary.Abs` AxisValue) 0.2)) (`GameplayStatics.GetWorldDeltaSeconds`) 2.0)))

(fn `UppdateControllerYaw`
  (if (>= (`self.CurrentForwardSpeed`) 100.0)
    (`self.AddControllerYawInput` (* (.yaw (`KismetMathLibrary.NormalizedDeltaRotator` (`self.K2_GetActorRotation`) (`self.GetControlRotation`))) (`GameplayStatics.GetWorldDeltaSeconds`)))))

(fn `UppdateLocalOffset`
  (params (DeltaSeconds :type "Float (double-precision)"))
  (`self.K2_AddActorLocalOffset` (`KismetMathLibrary.MakeVector` (* (`self.CurrentForwardSpeed`) DeltaSeconds) 0.0 (* (`self.CurrentUpSpeed`) DeltaSeconds))))

(fn `UppdateRotation`
  (`self.K2_AddActorLocalRotation` (`KismetMathLibrary.MakeRotator` (* (`self.CurrentRollSpeed`) (`GameplayStatics.GetWorldDeltaSeconds`)) (* (`self.CurentPitchSpeed`) (`GameplayStatics.GetWorldDeltaSeconds`)) (* (`self.CurrentYawSpeed`) (`GameplayStatics.GetWorldDeltaSeconds`)))))

(fn `UserConstructionScript`)

(fn `VerticalMove`
  (params (UpAxis :type "Float (double-precision)") (DownAxis :type "Float (double-precision)"))
  (bind _enginepow (`self.EnginePow`))
  (set `self.CurrentUpSpeed` (`KismetMathLibrary.FInterpTo` (`self.CurrentUpSpeed`) (+ (* UpAxis _enginepow) (* (* DownAxis -1.0) _enginepow)) (`GameplayStatics.GetWorldDeltaSeconds`) 2.0)))
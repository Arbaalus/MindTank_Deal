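; BP_WeaponsLibrary is a lookup library that maps weapon-related enums to their data.
; GetWeaponsInfo switches on weapon type to return the Blueprint class and display name for the revolver, machine gun, shotgun and grenade launcher.
; GetWeaponPartImage switches on an eight-entry part type enum with unnamed enumerators, but its branches show no returned image values.
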(fn `GetWeaponPartImage`
  (params (PartType :type Byte :default 0))
  (returns (Image :type "Texture Object Reference"))
  (switch `|SwitchEnum` PartType
    (:`NewEnumerator0`
      (return null))
    (:`NewEnumerator1`
      (return null))
    (:`NewEnumerator2`
      (return null))
    (:`NewEnumerator3`
      (return null))
    (:`NewEnumerator4`
      (return null))
    (:`NewEnumerator5`
      (return null))
    (:`NewEnumerator6`
      (return null))
    (:`NewEnumerator7`
      (return null))))

(fn `GetWeaponsInfo`
  (params (WeaponType :type "/Game/MurratProj/Blueprint/Weapons/E_WeaponType Enum" :default "NewEnumerator0"))
  (returns (WeaponInfo :type "/Game/MurratProj/Blueprint/Weapons/Struct_Weapon Structure"))
  (switch `/Game/MurratProj/Blueprint/Weapons/E_WeaponType` WeaponType
    (:`NewEnumerator0`
      (return (make `/Game/MurratProj/Blueprint/Weapons/Struct_Weapon` null "/Game/MurratProj/Blueprint/Weapons/Gun/BP_BaseGun.BP_BaseGun_C" "Revolver")))
    (:`NewEnumerator1`
      (return (make `/Game/MurratProj/Blueprint/Weapons/Struct_Weapon` null "/Game/MurratProj/Blueprint/Weapons/Gun/BP_BaseRifle.BP_BaseRifle_C" "Machine Gun")))
    (:`NewEnumerator2`
      (return (make `/Game/MurratProj/Blueprint/Weapons/Struct_Weapon` null "/Game/MurratProj/Blueprint/Weapons/Gun/BP_Shotgun.BP_Shotgun_C" "Shotgun")))
    (:`NewEnumerator3`
      (return (make `/Game/MurratProj/Blueprint/Weapons/Struct_Weapon` null "/Game/MurratProj/Blueprint/Weapons/Gun/BP_GrenadeLauncher.BP_GrenadeLauncher_C" "Grenade Launcher")))))
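; BP_BaseGun is a base gun Blueprint that fires projectiles with a cooldown, gunshot FX and sound.
; FireFunct traces from the pawn's ShootCam along its forward vector, then aims the spawn rotation from ShootDir at the hit point or trace end.
; SpawnBullet spawns ProjectilesClass with that rotation; its ignore-owner collision step is never executed.
; CurrentAmmo is initialized on BeginPlay but firing neither checks nor decrements it.
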(event `self.ReceiveBeginPlay`
  (set `self.CurrentAmmo` (`self.StartAmmo`)))

(event `self.ReceiveTick`
  (params (DeltaSeconds :type "Float (single-precision)"))
  (set `self.FireCooldown` (- (`self.FireCooldown`) DeltaSeconds)))

(event `self.ReceiveDestroyed`
  (`GameplayStatics.PlaySound2D` "/Game/MurratProj/Sound/Weapons/SFX_WeaponDestroyed.SFX_WeaponDestroyed" 1.0 1.0 0.0 null null))

(fn `FireFunct`
  (params (Pawn :type "/Game/MurratProj/Blueprint/Character_BP/BP_Charac_Player Object Reference"))
  (locals (Target :type "Vector Structure" :default (0.0 0.0 0.0)))
  (bind _shootcam (`/Game/MurratProj/Blueprint/Character_BP/BP_Charac_Player.ShootCam` Pawn))
  (bind _returnvalue (`SceneComponent.K2_GetComponentLocation` _shootcam))
  (`/Engine/EditorBlueprintResources/StandardMacros.CompareFloat` (`self.FireCooldown`)
    (:`==`
      _)
    (:`<`
      _))
  (set `self.FireCooldown` (`self.FireRate`))
  (`ActorComponent.SetActive` (`self.FX_Gunshot`) true true)
  (`GameplayStatics.PlaySound2D` (`self.ShootingSound`) 1.0 1.0 0.0 null null)
  (bind (_outhit _returnvalue_2) (`KismetSystemLibrary.LineTraceSingle` _returnvalue (+ _returnvalue (* (`KismetMathLibrary.GetForwardVector` (`SceneComponent.K2_GetComponentRotation` _shootcam)) 10000.0)) "TraceTypeQuery1" true (`|MakeArray` (`self.GetOwner`))))
  (if _returnvalue_2
    (bind _output_get (set `local.Target` (`.Location` (`GameplayStatics.BreakHitResult` _outhit))))
    (else
      (set `local.Target` (`.TraceEnd` (`GameplayStatics.BreakHitResult` _outhit)))))
  (`self.SpawnBullet` (`KismetMathLibrary.FindLookAtRotation` (`SceneComponent.K2_GetComponentLocation` (`self.ShootDir`)) _output_get)))

(fn `SpawnBullet`
  (params (Rot :type "Rotator Structure"))
  (`|SpawnActorFromClass` (`self.ProjectilesClass`) (`KismetMathLibrary.MakeTransform` (`SceneComponent.K2_GetComponentLocation` (`self.ShootDir`)) Rot) "AlwaysSpawn" "MultiplyWithRoot" null null))

(fn `UserConstructionScript`
  (set `self.WeaponMesh` (`StaticMeshComponent.StaticMesh` (`self.38Gun`))))
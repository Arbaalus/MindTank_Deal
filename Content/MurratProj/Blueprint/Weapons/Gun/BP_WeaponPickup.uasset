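; BP_WeaponPickup is a world pickup that gives the player a weapon of a configurable WeaponClass.
; On BeginPlay it copies the weapon mesh from that class's defaults onto its display mesh.
; When the player overlaps its sphere, it spawns the weapon, attaches it to the WeapSok socket, sets the player's current weapon and rifle flags, then destroys itself.
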(event `self.ReceiveBeginPlay`
  (`StaticMeshComponent.SetStaticMesh` (`self.WeaponMesh`) (`.WeaponMesh` (defaults `Object` (`self.WeaponClass`)))))

(event `self.Sphere.OnComponentBeginOverlap`
  (params (OverlappedComponent :type "PrimitiveComponent Object Reference") (OtherActor :type "Actor Object Reference") (OtherComp :type "PrimitiveComponent Object Reference") (OtherBodyIndex :type Integer) (bFromSweep :type Boolean) (SweepResult :type "HitResult Structure (by ref)"))
  (bind _asbp_charac_player_final_b (cast `/Game/MurratProj/Blueprint/Character_BP/BP_Charac_Player_FinalB` OtherActor))
  (`self.PickUp` _asbp_charac_player_final_b)
  (`self.K2_DestroyActor`))

(fn `PickUp`
  (params (Player :type "/Game/MurratProj/Blueprint/Character_BP/BP_Charac_Player_FinalB Object Reference"))
  (bind _returnvalue (`|SpawnActorFromClass` (`self.WeaponClass`) (`self.GetTransform`) "Undefined" "MultiplyWithRoot" null null))
  (bind _output_get (set `/Game/MurratProj/Blueprint/Character_BP/BP_Charac_Player_FinalB.CurrentWeapon` _returnvalue Player))
  (`self.K2_AttachToComponent` _output_get (`Character.Mesh` Player) "WeapSok" "SnapToTarget" "SnapToTarget" "KeepWorld" true)
  (set `/Game/MurratProj/Blueprint/Character_BP/BP_Charac_Player.isRiflle` (`.bSuccess` (cast `/Game/MurratProj/Blueprint/Weapons/Gun/BP_BaseRifle` _returnvalue :!pure true)) Player)
  (set `/Game/MurratProj/Blueprint/Character_BP/BP_Charac_Player.HasWeapon` true Player))

(fn `UserConstructionScript`)
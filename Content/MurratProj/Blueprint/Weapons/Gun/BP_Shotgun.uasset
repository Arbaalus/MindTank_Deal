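; BP_Shotgun is a shotgun weapon Blueprint that fires a spread of bullets per shot.
; It overrides SpawnBullet to call the parent implementation in a loop, once for each pellet.
; Each call rotates the aim's forward vector by random angles, up to 12.5 degrees either way, around its up and right axes.
; All other behavior comes from the parent class.
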(fn `SpawnBullet`
  (params (Rot :type "Rotator Structure"))
  (for _ (range 11)
    (`parent.SpawnBullet` (`KismetMathLibrary.MakeRotFromX` (`KismetMathLibrary.RotateAngleAxis` (`KismetMathLibrary.RotateAngleAxis` (`KismetMathLibrary.GetForwardVector` Rot) (`KismetMathLibrary.RandomFloatInRange` -12.5 12.5) (`KismetMathLibrary.GetUpVector` Rot)) (`KismetMathLibrary.RandomFloatInRange` -12.5 12.5) (`KismetMathLibrary.GetRightVector` Rot))))))

(fn `UserConstructionScript`
  (`parent.UserConstructionScript`))
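; EnnemiSpawner is an actor that spawns a batch of enemies for a mission and tracks how many are killed.
; StartSpawn places EnnemiNum actors of EnnemiType at random navigable points within its Sphere radius, giving each a reference back to the spawner.
; CheckKill counts kills until the batch is cleared, then EndMission waits briefly and tells the level's MissionManager to start a random mission.
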(event `self.ReceiveBeginPlay`
  (bind _returnvalue (`GameplayStatics.GetActorOfClass` "/Game/MurratProj/Blueprint/GameplayBP/MissionManager.MissionManager_C"))
  (set `self.Mission` _returnvalue))

(event `StartSpawn`
  (for _ (range 1 (+ (`self.EnnemiNum`) 1))
    (bind _randomlocation (`NavigationSystemV1.K2_GetRandomLocationInNavigableRadius` (`self.K2_GetActorLocation`) (`SphereComponent.GetScaledSphereRadius` (`self.Sphere`)) null null))
    (bind _returnvalue (`|SpawnActorFromClass` (`self.EnnemiType`) (`KismetMathLibrary.MakeTransform` (+ _randomlocation (0.0 0.0 88.0))) "AdjustIfPossibleButAlwaysSpawn" "MultiplyWithRoot" null null))
    (set `/Game/MurratProj/Blueprint/Character_BP/BP_Charac_Zombie.SpawnerRef` self _returnvalue)
    (`KismetSystemLibrary.PrintString` "Hello")))

(event `/Game/MurratProj/Blueprint/Character_BP/MissionInterface.CheckKill`
  (bind _playerkill (`self.PlayerKill`))
  (if (< _playerkill (- (`self.EnnemiNum`) 1))
    (`/Engine/EditorBlueprintResources/StandardMacros.IncrementInt` _playerkill)
    (else
      (`self.EndMission`)
      (set `self.PlayerKill` 0))))

(event `EndMission`
  (`KismetSystemLibrary.PrintString` "End Mission")
  (`KismetSystemLibrary.Delay` 5.0)
  (`/Game/MurratProj/Blueprint/GameplayBP/MissionManager.StartRandMission` (`self.Mission`)))

(fn `UserConstructionScript`)
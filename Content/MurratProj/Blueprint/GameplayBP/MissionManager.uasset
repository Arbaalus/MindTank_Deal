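; MissionManager is a Blueprint that starts missions by triggering enemy spawners.
; On BeginPlay it caches all EnnemiSpawner actors in the level, then calls StartSpawn on the FirstMission reference.
; StartRandMission calls StartSpawn on a randomly picked cached spawner; its only call within this graph is disconnected and never runs.
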(event `self.ReceiveBeginPlay`
  (bind _outactors (`GameplayStatics.GetAllActorsOfClass` "/Game/MurratProj/Blueprint/GameplayBP/EnnemiSpawner.EnnemiSpawner_C"))
  (set `self.Spawner` _outactors)
  (`/Game/MurratProj/Blueprint/GameplayBP/EnnemiSpawner.StartSpawn` (`self.FirstMission`)))

(event `StartRandMission`
  (`/Game/MurratProj/Blueprint/GameplayBP/EnnemiSpawner.StartSpawn` (`|GetArrayItem` (`self.Spawner`) (`KismetMathLibrary.RandomInteger` (`KismetArrayLibrary.Array_Length` (`self.Spawner`))))))

(fn `UserConstructionScript`)
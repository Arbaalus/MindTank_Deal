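; Player character Blueprint for a cat, with debug-style key bindings for triggering animations.
; G and H play the root-motion and in-place crouch attack clips directly on the Cat component through PlayAnimation, without looping.
; J sets IsJumping, which nothing in this Blueprint reads or clears.
; An unconnected fall-to-land animation sequence with a delay never runs, and the default events are disabled.
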(event `Key|G`
  (params (Key :type "Key Structure"))
  (:`Pressed`
    (`SkeletalMeshComponent.PlayAnimation` (`self.Cat`) "/Game/LowPoly_Cat/Animations/Anim_Cat_Attack_crouch_RM.Anim_Cat_Attack_crouch_RM" false)))

(event `Key|H`
  (params (Key :type "Key Structure"))
  (:`Pressed`
    (`SkeletalMeshComponent.PlayAnimation` (`self.Cat`) "/Game/LowPoly_Cat/Animations/Anim_Cat_Attack_crouch_IP.Anim_Cat_Attack_crouch_IP" false)))

(event `Key|J`
  (params (Key :type "Key Structure"))
  (:`Pressed`
    (set `self.IsJumping` true)))

(fn `UserConstructionScript`
  (`parent.UserConstructionScript`))
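; Player character with gun fire, melee, weapon switching, pause menu and enterable vehicles, driven by Enhanced Input.
; Fire shoots the current weapon or plays a smash montage without a gun; switching flip-flops it between two sockets on an equip montage notify.
; Interaction possesses a detected vehicle, moves and attaches the character to its seat socket, and passes handle transforms to the AnimBP.
; ExitCar detaches, moves to the left exit point and repossesses the character.
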(event `TriggerFire`
  (params (Weapon :type "/Game/MurratProj/Blueprint/Weapons/Gun/BP_BaseGun Object Reference"))
  (if (not (`self.InFire`))
    (set `self.InFire` true)
    (`|PlayMontage` (`self.Mesh`) "/Game/PolygonCity/Meshes/Characters/Animation/Fire_Rifle_Ironsights_Montage.Fire_Rifle_Ironsights_Montage"
      (:`then`
        (`/Game/MurratProj/Blueprint/Weapons/Gun/BP_BaseGun.FireFunct` Weapon self))
      (:`OnCompleted`
        (set `self.InFire` false)))))

(event `self.ReceiveBeginPlay`
  (`parent.ReceiveBeginPlay`))

(event `EnhancedInput|/Game/ThirdPerson/Input/Actions/Fire`
  (params (ActionValue :type Boolean) (ElapsedSeconds :type "Float (double-precision)") (TriggeredSeconds :type "Float (double-precision)") (InputAction :type "InputAction Object Reference" :default "/Game/ThirdPerson/Input/Actions/Fire.Fire"))
  (:`Triggered`
    (bind _currentweapon (`self.CurrentWeapon`)
      (:`then`
        (if (`self.GunOn`)
          (`/Game/MurratProj/Blueprint/Weapons/Gun/BP_BaseGun.FireFunct` _currentweapon self)))
      (:`else`)))
  (:`Started`
    (if (not (`self.GunOn`))
      (`|PlayMontage` (`self.Mesh`) "/Game/PolygonCity/Meshes/Characters/Animation/Smash_Montage.Smash_Montage"))))

(event `EnhancedInput|/Game/ThirdPerson/Input/Actions/SwitchWeapon`
  (params (ActionValue :type Boolean) (ElapsedSeconds :type "Float (double-precision)") (TriggeredSeconds :type "Float (double-precision)") (InputAction :type "InputAction Object Reference" :default "/Game/ThirdPerson/Input/Actions/SwitchWeapon.SwitchWeapon"))
  (:`Started`
    (`|PlayMontage` (`self.Mesh`) "/Game/PolygonCity/Meshes/Characters/Animation/Equip_Pistol_Standing_Montage.Equip_Pistol_Standing_Montage"
      (:`OnNotifyBegin`
        (`/Engine/EditorBlueprintResources/StandardMacros.FlipFlop`
          (:`A`
            (`self.EquipWeapon` false))
          (:`B`
            (`self.EquipWeapon` true)))))))

(event `EnhancedInput|/Game/ThirdPerson/Input/Actions/IA_Pause`
  (params (ActionValue :type Boolean) (ElapsedSeconds :type "Float (double-precision)") (TriggeredSeconds :type "Float (double-precision)") (InputAction :type "InputAction Object Reference" :default "/Game/ThirdPerson/Input/Actions/IA_Pause.IA_Pause"))
  (:`Started`
    (`/Engine/EditorBlueprintResources/StandardMacros.DoOnce` false :!label _label
      (:`Completed`
        (bind _returnvalue (`|CreateWidget` "/Game/MurratProj/Widgets/PauseMenu.PauseMenu_C"))
        (`UserWidget.AddToViewport` _returnvalue 0)
        (`GameplayStatics.SetGamePaused` true)))))

(event `ResetPause`
  (goto _label :!via `Reset`))

(event `EnhancedInput|/Game/ThirdPerson/Input/Actions/IA_Interaction`
  (params (ActionValue :type Boolean) (ElapsedSeconds :type "Float (double-precision)") (TriggeredSeconds :type "Float (double-precision)") (InputAction :type "InputAction Object Reference" :default "/Game/ThirdPerson/Input/Actions/IA_Interaction.IA_Interaction"))
  (:`Started`
    (if (`self.DetectCar`)
      (`Controller.Possess` (`GameplayStatics.GetPlayerController` 0) (`self.Vehicle`))
      (`self.EnterCar`))))

(event `self.ReceivePossessed`
  (params (NewController :type "Controller Object Reference"))
  (message `EnhancedInputSubsystemInterface.AddMappingContext` (pcsubsystem `EnhancedInputLocalPlayerSubsystem` (`GameplayStatics.GetPlayerController` 0)) "/Game/ThirdPerson/Input/IMC_Default.IMC_Default" 0 (struct)))

(event `self.ReceiveUnpossessed`
  (params (OldController :type "Controller Object Reference"))
  (message `EnhancedInputSubsystemInterface.RemoveMappingContext` (pcsubsystem `EnhancedInputLocalPlayerSubsystem` (`GameplayStatics.GetPlayerController` 0)) "/Game/ThirdPerson/Input/IMC_Default.IMC_Default" (struct)))

(event `EnterCar`
  (bind _vehicle (`self.Vehicle`))
  (bind _mesh (`WheeledVehiclePawn.Mesh` (`self.Vehicle`)))
  (bind _mesh_2 (`WheeledVehiclePawn.Mesh` (`self.Vehicle`)))
  (`PrimitiveComponent.SetCollisionEnabled` (`self.CapsuleComponent`) "NoCollision")
  (`AnimInstance.Montage_Play` (`SkeletalMeshComponent.GetAnimInstance` (`self.Mesh`)) "/Game/PolygonCity/Meshes/Characters/Animation/Enter_BikeLeft_Montage.Enter_BikeLeft_Montage" 1.0 "MontageLength" 0.0 true)
  (`KismetSystemLibrary.MoveComponentTo` (`self.CapsuleComponent`) (`SceneComponent.GetSocketLocation` _mesh_2 "Sit") (`SceneComponent.GetSocketRotation` _mesh_2 "Sit") false false 1.0 true)
  (`self.K2_AttachToActor` (`self.Vehicle`) "Sit" "KeepWorld" "KeepWorld" "KeepRelative")
  (set `self.InCar` true)
  (set `/Game/MurratProj/Blueprint/Vehicle/BP_BaseVehicle.EngineOn` true _vehicle)
  (bind _assynty_anim_bp (cast `/Game/MurratProj/Animation/AnimBp/Synty_AnimBP` (`SkeletalMeshComponent.GetAnimInstance` (`self.Mesh`))))
  (bind _output_get (set `/Game/MurratProj/Blueprint/Vehicle/BP_BaseVehicle.Anim BP` _assynty_anim_bp _vehicle))
  (set `/Game/MurratProj/Animation/AnimBp/Synty_AnimBP.Vehicle` (`/Game/MurratProj/Blueprint/Vehicle/BP_BaseVehicle.VehicleType` _vehicle) _output_get)
  (set `/Game/MurratProj/Animation/AnimBp/Synty_AnimBP.DriveHandL` (`SceneComponent.GetSocketTransform` _mesh "HandleLeft" "RTS_World") _assynty_anim_bp)
  (set `/Game/MurratProj/Animation/AnimBp/Synty_AnimBP.DriveHandR` (`SceneComponent.GetSocketTransform` _mesh "HandleRight" "RTS_World") _assynty_anim_bp))

(event `ExitCar`
  (bind _exitleftcollision (`/Game/MurratProj/Blueprint/Vehicle/BP_BaseVehicle.ExitLeftCollision` (`self.Vehicle`)))
  (bind (_returnvalue_roll _returnvalue_pitch _returnvalue_yaw) (`KismetMathLibrary.BreakRotator` (`SceneComponent.K2_GetComponentRotation` _exitleftcollision)))
  (set `/Game/MurratProj/Blueprint/Vehicle/BP_BaseVehicle.EngineOn` false (`self.Vehicle`))
  (`AnimInstance.Montage_Play` (`SkeletalMeshComponent.GetAnimInstance` (`self.Mesh`)) "/Game/PolygonCity/Meshes/Characters/Animation/Exit_BikeLeft_Montage.Exit_BikeLeft_Montage" 1.0 "MontageLength" 0.0 true)
  (`self.K2_DetachFromActor` "KeepWorld" "KeepWorld" "KeepWorld")
  (`KismetSystemLibrary.MoveComponentTo` (`self.CapsuleComponent`) (`SceneComponent.K2_GetComponentLocation` _exitleftcollision) (`KismetMathLibrary.MakeRotator` 0.0 0.0 _returnvalue_yaw) false false 0.8 true)
  (`PrimitiveComponent.SetCollisionEnabled` (`self.CapsuleComponent`) "QueryAndPhysics")
  (`Controller.Possess` (`GameplayStatics.GetPlayerController` 0) self)
  (set `self.InCar` false))

(event `/Game/MurratProj/Blueprint/Character_BP/Hit_Interface.NotifyKill`
  (`KismetSystemLibrary.PrintString` "Kill"))

(fn `AttachPlayerToVehicle`
  (bind _capsulecomponent (`self.CapsuleComponent`))
  (`self.K2_AttachToActor` (`self.Vehicle`) "Sit" "SnapToTarget" "SnapToTarget" "KeepRelative")
  (`self.K2_SetActorRelativeRotation` (struct :`Yaw` 90.0))
  (`PrimitiveComponent.SetCollisionResponseToChannel` _capsulecomponent "ECC_Pawn" "ECR_Ignore")
  (`PrimitiveComponent.SetCollisionResponseToChannel` _capsulecomponent "ECC_Vehicle" "ECR_Ignore")
  (set `self.InCar` true))

(fn `EquipWeapon`
  (params (Equip :type Boolean))
  (if Equip
    (bind _currentweapon (`self.CurrentWeapon`)
      (:`then`
        (`self.K2_AttachToComponent` _currentweapon (`self.Mesh`) "WeapSok" "SnapToTarget" "SnapToTarget" "KeepRelative" true)
        (set `self.HasWeapon` true))
      (:`else`))
    (else
      (bind _currentweapon_2 (`self.CurrentWeapon`)
        (:`then`
          (`self.K2_AttachToComponent` _currentweapon_2 (`self.Mesh`) "RifleSock" "SnapToTarget" "SnapToTarget" "KeepRelative" true)
          (set `self.HasWeapon` false))
        (:`else`)))))

(fn `UserConstructionScript`
  (`parent.UserConstructionScript`))
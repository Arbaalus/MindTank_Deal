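; Pedestrian spawner that populates the navmesh around the player with AI pedestrians, capped at a spawn limit.
; A looping one-second timer spawns a pedestrian at a random navigable point within a randomized radius of the player, at fixed height, and tracks it.
; Invalid entries are pruned from the tracked array only once the limit is reached.
; A player-proximity helper function exists but is not called here.
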(event `self.ReceiveBeginPlay`
  (bind _returnvalue (`KismetSystemLibrary.K2_SetTimerDelegate` (delegate `SpawnPedestrian`) 1.0 true))
  (set `self.TimerHandle` _returnvalue))

(event `SpawnPedestrian`
  (if (< (`KismetArrayLibrary.Array_Length` (`self.SpawnedPawns`)) (`self.SpawnLimit`))
    (bind _randomlocation (`NavigationSystemV1.K2_GetRandomLocationInNavigableRadius` (`self.K2_GetActorLocation` (`GameplayStatics.GetPlayerCharacter` 0)) (`KismetMathLibrary.RandomFloatInRange` (`self.SpawnDistanceMin`) (`self.SpawnDistanceMax`)) null null))
    (bind _returnvalue (`AIBlueprintHelperLibrary.SpawnAIFromClass` "/Game/MurratProj/Blueprint/Character_BP/Pedestrians/BP_Charac_Pedestrian.BP_Charac_Pedestrian_C" null (`KismetMathLibrary.MakeVector` (.x _randomlocation) (.y _randomlocation) 100.0) (struct) true null))
    (`KismetArrayLibrary.Array_Add` (`self.SpawnedPawns`) _returnvalue)
    (else
      (for _array_element (`self.SpawnedPawns`)
        (if (not (`KismetSystemLibrary.IsValid` _array_element))
          (`KismetArrayLibrary.Array_RemoveItem` (`self.SpawnedPawns`) _array_element)
          (`KismetSystemLibrary.PrintString` "Removed element"))))))

(fn `IsPlayerNearSpawner`
  (params (DistanceToCheck :type "Float (double-precision)"))
  (returns (ReturnValue :type Boolean))
  (return (< (`self.GetDistanceTo` (`GameplayStatics.GetPlayerPawn` 0) self) DistanceToCheck)))

(fn `UserConstructionScript`)
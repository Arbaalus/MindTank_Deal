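; Pedestrian character that roams the navmesh, with a random mesh, walk speed and health set in the Construction Script.
; Roaming chains random AI MoveTo destinations, and a looping timer destroys the actor when far from the player.
; Bumps from BP_Charac_Base play a random hit montage and sometimes trigger a temporary run.
; Dying handles montage, sound, blood decal and player kill notification; its vehicle-impact trigger is disconnected.
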(event `self.ReceiveBeginPlay`
  (`parent.ReceiveBeginPlay`)
  (`KismetSystemLibrary.K2_SetTimerDelegate` (delegate `DestroyIfPlayerIsTooFar`) 1.0 true))

(event `DestroyIfPlayerIsTooFar`
  (if (`self.IsPlayerFar` (`self.DestroyAtDistanceFromPlayer`))
    (`self.K2_DestroyActor`)))

(event `self.Roaming`
  (if (`|EnumEquality` (`self.States`) "NewEnumerator0")
    (bind _randomlocation (`NavigationSystemV1.K2_GetRandomLocationInNavigableRadius` (`self.K2_GetActorLocation`) 4000.0 null null))
    (`|AIMoveTo` (`AIBlueprintHelperLibrary.GetAIController` self) null _randomlocation null
      (:`OnSuccess`
        (`KismetSystemLibrary.Delay` 2.0)
        (`self.Roaming`))
      (:`OnFail`
        (`self.Roaming`)))))

(event `self.CapsuleComponent.OnComponentHit`
  (params (HitComponent :type "PrimitiveComponent Object Reference") (OtherActor :type "Actor Object Reference") (OtherComp :type "PrimitiveComponent Object Reference") (NormalImpulse :type "Vector Structure") (Hit :type "HitResult Structure (by ref)"))
  (cast `/Game/MurratProj/Blueprint/Character_BP/BP_Charac_Base` OtherActor)
  (`/Engine/EditorBlueprintResources/StandardMacros.DoOnce` false :!label _label
    (:`Completed`
      (`|PlayMontage` (`self.Mesh`) "/Game/PolygonCity/Meshes/Characters/Animation/WalkProAnim_Root/Sword_Hit_L_1_Montage.Sword_Hit_L_1_Montage" 1.0 0.0 (select `int` (`KismetMathLibrary.RandomInteger` 4) :`0` "Hit1" :`1` "Hit2" :`2` "Hit3" :`3` "Hit4" :!type "Name")
        (:`then`
          (if (`KismetMathLibrary.RandomBool`)
            (`self.RunSomewhere`)
            (`KismetSystemLibrary.Delay` 5.0)
            (`self.DefineWalkingSpeed`)))
        (:`OnCompleted`
          (goto _label :!via `Reset`))
        (:`OnInterrupted`
          (goto _label :!via `Reset`))))))

(fn `DefineWalkingSpeed`
  (set `CharacterMovementComponent.MaxWalkSpeed` (`KismetMathLibrary.SelectFloat` (`self.MinWalkingSpeed`) (`self.MaxWalkingSpeed`) (`KismetMathLibrary.RandomBool`)) (`self.CharacterMovement`)))

(fn `Dying`
  (bind _returnvalue (`KismetMathLibrary.RandomFloatInRange` 0.0 360.0))
  (set `self.IsDie` true)
  (`AnimInstance.Montage_Play` (`SkeletalMeshComponent.GetAnimInstance` (`self.Mesh`)) "/Game/MurratProj/Animation/Anim_Sample/ZonbieMove/zombie_death_Montage.zombie_death_Montage" 1.0 "MontageLength" 0.0 true)
  (`GameplayStatics.PlaySoundAtLocation` "/Game/MurratProj/Sound/Character_pain.Character_pain" (`self.K2_GetActorLocation`) (struct) 1.0 1.0 0.0 null null null null)
  (`MovementComponent.StopMovementImmediately` (`self.CharacterMovement`))
  (`Controller.StopMovement` (`AIBlueprintHelperLibrary.GetAIController` self))
  (`PrimitiveComponent.SetCollisionEnabled` (`self.CapsuleComponent`) "NoCollision")
  (message `/Game/MurratProj/Blueprint/Character_BP/Hit_Interface.NotifyKill` (`GameplayStatics.GetPlayerCharacter` 0) (`GameplayStatics.GetObjectClass` self) (`self.EnnemiValue`))
  (`GameplayStatics.SpawnDecalAtLocation` "/Game/MurratProj/Textures/Environment/Material/M_DecalBlood01.M_DecalBlood01" (32.0 128.0 128.0) (- (`self.K2_GetActorLocation`) (`KismetMathLibrary.MakeVector` 0.0 0.0 (`.OutHalfHeight` (`CapsuleComponent.GetScaledCapsuleSize` (`self.CapsuleComponent`))))) (`KismetMathLibrary.MakeRotator` _returnvalue -90.0 _returnvalue))
  (`Controller.UnPossess` (`self.GetController`)))

(fn `IsPlayerFar`
  (params (DistanceToCheck :type "Float (double-precision)"))
  (returns (ReturnValue :type Boolean))
  (return (> (`self.GetDistanceTo` (`GameplayStatics.GetPlayerPawn` 0) self) DistanceToCheck)))

(fn `RunSomewhere`
  (set `CharacterMovementComponent.MaxWalkSpeed` (`self.RunningSpeed`) (`self.CharacterMovement`))
  (`self.Roaming`))

(fn `UserConstructionScript`
  (`self.DefineWalkingSpeed`)
  (set `SkeletalMeshComponent.SkeletalMeshAsset` (select `int` (`KismetMathLibrary.RandomInteger` 20) :`0` "/Game/PolygonCity/Meshes/Characters/SK_Character_BusinessMan_Shirt.SK_Character_BusinessMan_Shirt" :`1` "/Game/PolygonTown/Meshes/Characters/SK_Character_Father_01.SK_Character_Father_01" :`2` "/Game/PolygonTown/Meshes/Characters/SK_Character_Father_02.SK_Character_Father_02" :`3` "/Game/PolygonTown/Meshes/Characters/SK_Character_Mother_01.SK_Character_Mother_01" :`4` "/Game/PolygonTown/Meshes/Characters/SK_Character_Mother_02.SK_Character_Mother_02" :`5` "/Game/PolygonCityChar/Characters/SK_Character_PunkGuy.SK_Character_PunkGuy" :`6` "/Game/PolygonCityChar/Characters/SK_Character_Tourist.SK_Character_Tourist" :`7` "/Game/PolygonTown/Meshes/Characters/SK_Character_Son_01.SK_Character_Son_01" :`8` "/Game/PolygonTown/Meshes/Characters/SK_Character_Daughter_01.SK_Character_Daughter_01" :`9` "/Game/Polygon_BattleRoyale/Meshes/Characters/SK_Chr_RedneckMale_01.SK_Chr_RedneckMale_01" :`10` "/Game/PolygonTown/Meshes/Characters/SK_Character_SchoolBoy_01.SK_Character_SchoolBoy_01" :`11` "/Game/PolygonTown/Meshes/Characters/SK_Character_SchoolGirl_01.SK_Character_SchoolGirl_01" :`12` "/Game/PolygonCityChar/Characters/SK_Character_HipsterGirl.SK_Character_HipsterGirl" :`13` "/Game/PolygonCity/Meshes/Characters/SK_Character_BusinessMan_Shirt.SK_Character_BusinessMan_Shirt" :`14` "/Game/PolygonCity/Meshes/Characters/SK_Character_Male_Hoodie.SK_Character_Male_Hoodie" :`15` "/Game/PolygonTown/Meshes/Characters/SK_Character_ShopKeeper_01.SK_Character_ShopKeeper_01" :`16` "/Game/PolygonCityChar/Characters/SK_Character_ShopKeeper.SK_Character_ShopKeeper" :`17` "/Game/PolygonCity/Meshes/Characters/SK_Character_BusinessMan_Shirt.SK_Character_BusinessMan_Shirt" :`18` "/Game/PolygonCityChar/Characters/SK_Character_FastFoodGuy.SK_Character_FastFoodGuy" :`19` "/Game/PolygonCityChar/Characters/SK_Character_Hotdog.SK_Character_Hotdog" :!type "SkeletalMesh Object Reference") (`self.Mesh`))
  (set `self.Health` (`KismetMathLibrary.RandomFloatInRange` (`self.PedestrianMinHealth`) (`self.PedestrianMaxHealth`))))
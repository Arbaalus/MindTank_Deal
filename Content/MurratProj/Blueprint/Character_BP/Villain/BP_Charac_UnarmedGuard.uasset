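; Unarmed guard villain character that extends a parent Blueprint with randomized looks and movement speeds.
; On construction it picks one of two male skeletal meshes at random, sets Health from GuardHealth, and randomly chooses either the minimum or maximum walking speed.
; The MovetoTarget event switches movement to RunSpeed before calling the parent's move logic.
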(event `self.MoveToTarget`
  (set `CharacterMovementComponent.MaxWalkSpeed` (`self.RunSpeed`) (`self.CharacterMovement`))
  (`parent.MoveToTarget`))

(fn `DefineWalkingSpeed`
  (set `CharacterMovementComponent.MaxWalkSpeed` (`KismetMathLibrary.SelectFloat` (`self.MinWalkingSpeed`) (`self.MaxWalkingSpeed`) (`KismetMathLibrary.RandomBool`)) (`self.CharacterMovement`)))

(fn `UserConstructionScript`
  (`parent.UserConstructionScript`)
  (set `SkeletalMeshComponent.SkeletalMeshAsset` (select `int` (`KismetMathLibrary.RandomInteger` 2) :`0` "/Game/Polygon_BattleRoyale/Meshes/Characters/SK_Chr_ToplessMale_01.SK_Chr_ToplessMale_01" :`1` "/Game/Polygon_BattleRoyale/Meshes/Characters/SK_Chr_MercenaryMale_01.SK_Chr_MercenaryMale_01" :!type "SkeletalMesh Object Reference") (`self.Mesh`))
  (set `self.Health` (`self.GuardHealth`))
  (`self.DefineWalkingSpeed`))
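; BP_Charac_Hobo is a hobo villain character Blueprint that randomizes its appearance whenever it is constructed.
; The Construction Script picks random array entries for body mesh, first material slot, hair, beard, hat and the Beer component's weapon mesh.
; RandMeshBodyInt is stored from a separate random roll, so it need not match the chosen body.
; The event graph holds only disabled default events, so no gameplay logic is defined here.
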(fn `UserConstructionScript`
  (locals (RandBeard_Int :type Integer :default 0))
  (bind _randmeshbody (`self.RandMeshBody`))
  (bind _randmaterial (`self.RandMaterial`))
  (bind _randweapon (`self.RandWeapon`))
  (bind _randhat (`self.RandHat`))
  (bind _randhair (`self.RandHair`))
  (bind _randbeard (`self.RandBeard`))
  (bind _returnvalue (`KismetMathLibrary.RandomInteger` (`KismetArrayLibrary.Array_Length` _randmeshbody)))
  (`SkeletalMeshComponent.SetSkeletalMeshAsset` (`self.Mesh`) (`|GetArrayItem` _randmeshbody _returnvalue))
  (set `self.RandMeshBody-Int` _returnvalue)
  (`PrimitiveComponent.SetMaterial` (`self.Mesh`) 0 (`|GetArrayItem` _randmaterial (`KismetMathLibrary.RandomInteger` (`KismetArrayLibrary.Array_Length` _randmaterial))))
  (`StaticMeshComponent.SetStaticMesh` (`self.Beer`) (`|GetArrayItem` _randweapon (`KismetMathLibrary.RandomInteger` (`KismetArrayLibrary.Array_Length` _randweapon))))
  (`StaticMeshComponent.SetStaticMesh` (`self.Hair`) (`|GetArrayItem` _randhair (`KismetMathLibrary.RandomInteger` (`KismetArrayLibrary.Array_Length` _randhair))))
  (`StaticMeshComponent.SetStaticMesh` (`self.Beard`) (`|GetArrayItem` _randbeard (`KismetMathLibrary.RandomInteger` (`KismetArrayLibrary.Array_Length` _randbeard))))
  (`StaticMeshComponent.SetStaticMesh` (`self.Hat`) (`|GetArrayItem` _randhat (`KismetMathLibrary.RandomInteger` (`KismetArrayLibrary.Array_Length` _randhat)))))
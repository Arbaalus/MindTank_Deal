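; BP_Charac_SDF is a villain character child Blueprint that spawns as a randomized, beer-carrying redneck or topless male.
; The construction script randomizes body mesh, material and alcohol prop (three bottle meshes across four rolls), then sets Health from GuardHealth.
; DefineWalkingSpeed randomly picks either the minimum or maximum walking speed.
; MovetoTarget switches to RunSpeed before calling the parent's movement logic, which is the only active event here.
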(event `self.MoveToTarget`
  (set `CharacterMovementComponent.MaxWalkSpeed` (`self.RunSpeed`) (`self.CharacterMovement`))
  (`parent.MoveToTarget`))

(fn `DefineWalkingSpeed`
  (set `CharacterMovementComponent.MaxWalkSpeed` (`KismetMathLibrary.SelectFloat` (`self.MinWalkingSpeed`) (`self.MaxWalkingSpeed`) (`KismetMathLibrary.RandomBool`)) (`self.CharacterMovement`)))

(fn `UserConstructionScript`
  (`SkeletalMeshComponent.SetSkeletalMeshAsset` (`self.Mesh`) (select `int` (`KismetMathLibrary.RandomInteger` 2) :`0` "/Game/Polygon_BattleRoyale/Meshes/Characters/SK_Chr_RedneckMale_01.SK_Chr_RedneckMale_01" :`1` "/Game/Polygon_BattleRoyale/Meshes/Characters/SK_Chr_ToplessMale_01.SK_Chr_ToplessMale_01" :!type "SkeletalMesh Object Reference"))
  (`PrimitiveComponent.SetMaterial` (`self.Mesh`) 0 (select `int` (`KismetMathLibrary.RandomInteger` 4) :`0` "/Game/Polygon_BattleRoyale/Materials/Mat_PolygonBattleRoyale_01_A.Mat_PolygonBattleRoyale_01_A" :`1` "/Game/Polygon_BattleRoyale/Materials/Mat_PolygonBattleRoyale_02_A.Mat_PolygonBattleRoyale_02_A" :`2` "/Game/Polygon_BattleRoyale/Materials/Mat_PolygonBattleRoyale_03_A.Mat_PolygonBattleRoyale_03_A" :`3` "/Game/Polygon_BattleRoyale/Materials/Mat_PolygonBattleRoyale_04_A.Mat_PolygonBattleRoyale_04_A" :!type "MaterialInterface Object Reference"))
  (`StaticMeshComponent.SetStaticMesh` (`self.Beer`) (select `int` (`KismetMathLibrary.RandomInteger` 4) :`0` "/Game/PolygonTown/Meshes/Items/SM_Item_Alcohol_01.SM_Item_Alcohol_01" :`1` "/Game/PolygonTown/Meshes/Items/SM_Item_Alcohol_02.SM_Item_Alcohol_02" :`2` "/Game/PolygonTown/Meshes/Items/SM_Item_Alcohol_03.SM_Item_Alcohol_03" :!type "StaticMesh Object Reference"))
  (set `self.Health` (`self.GuardHealth`))
  (`self.DefineWalkingSpeed`))
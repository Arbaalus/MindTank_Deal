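; BP_Charac_Base is a base character Blueprint that handles health and death.
; AnyDamage feeds HealthFunct, which subtracts damage and calls PawnHit while health stays above zero, or zeroes health and calls Dying once.
; Dying only sets the IsDie flag, which guards against repeated deaths, and NotifyKill is an empty event.
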(event `self.ReceiveAnyDamage`
  (params (Damage :type "Float (single-precision)") (DamageType :type "DamageType Object Reference") (InstigatedBy :type "Controller Object Reference") (DamageCauser :type "Actor Object Reference"))
  (`self.HealthFunct` Damage))

(event `/Game/MurratProj/Blueprint/Character_BP/Hit_Interface.NotifyKill`
  (params (EnnemieClass :type "/Game/MurratProj/Blueprint/Character_BP/BP_Charac_Zombie Class Reference") (EnnemieValue :type Integer)))

(fn `Dying`
  (set `self.IsDie` true))

(fn `HealthFunct`
  (params (Damage :type "Float (double-precision)"))
  (bind _returnvalue (- (`self.Health`) Damage))
  (if (and (> _returnvalue 0.0) (not (`self.IsDie`)))
    (set `self.Health` _returnvalue)
    (`self.PawnHit` 0.0)
    (else
      (set `self.Health` 0.0)
      (if (not (`self.IsDie`))
        (`self.Dying`)))))

(fn `UserConstructionScript`)
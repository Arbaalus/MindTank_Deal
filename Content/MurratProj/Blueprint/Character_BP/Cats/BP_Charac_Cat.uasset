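; Cat character Blueprint that gives each cat a random breed or coat appearance.
; The construction script calls DefineWalkingSpeed, picks a skeletal mesh through a random-index Select and sets a fixed starting Health.
; One of the sixteen Select slots is empty, so a roll can leave the cat without a mesh.
; The event graph holds only disabled default events.
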(fn `UserConstructionScript`
  (`self.DefineWalkingSpeed`)
  (set `SkeletalMeshComponent.SkeletalMeshAsset` (select `int` (`KismetMathLibrary.RandomInteger` 16) :`0` "/Game/LowPoly_Cat/Meshes/Mesh_Cat_Abyss.Mesh_Cat_Abyss" :`1` "/Game/LowPoly_Cat/Meshes/Mesh_Cat_black.Mesh_Cat_black" :`2` "/Game/LowPoly_Cat/Meshes/Mesh_Cat_Black_White.Mesh_Cat_Black_White" :`3` "/Game/LowPoly_Cat/Meshes/Mesh_Cat_Blue.Mesh_Cat_Blue" :`4` "/Game/LowPoly_Cat/Meshes/Mesh_Cat_Bobtail.Mesh_Cat_Bobtail" :`5` "/Game/LowPoly_Cat/Meshes/Mesh_Cat_Brit.Mesh_Cat_Brit" :`6` "/Game/LowPoly_Cat/Meshes/Mesh_Cat_brown.Mesh_Cat_brown" :`7` "/Game/LowPoly_Cat/Meshes/Mesh_Cat_cream.Mesh_Cat_cream" :`8` "/Game/LowPoly_Cat/Meshes/Mesh_Cat_maine.Mesh_Cat_maine" :`9` "/Game/LowPoly_Cat/Meshes/Mesh_Cat_Pers.Mesh_Cat_Pers" :`10` "/Game/LowPoly_Cat/Meshes/Mesh_Cat_Red.Mesh_Cat_Red" :`11` null :`12` "/Game/LowPoly_Cat/Meshes/Mesh_Cat_Red_White.Mesh_Cat_Red_White" :`13` "/Game/LowPoly_Cat/Meshes/Mesh_Cat_Siamese.Mesh_Cat_Siamese" :`14` "/Game/LowPoly_Cat/Meshes/Mesh_Cat_Sphynx.Mesh_Cat_Sphynx" :`15` "/Game/LowPoly_Cat/Meshes/Mesh_Cat_white.Mesh_Cat_white" :!type "SkeletalMesh Object Reference") (`self.Mesh`))
  (set `self.Health` 5.0))
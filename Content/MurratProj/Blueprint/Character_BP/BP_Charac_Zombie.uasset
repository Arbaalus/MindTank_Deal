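; Zombie enemy character that roams random navigable points until pawn sensing spots the player, then chases and punches in melee range.
; A state enum drives the move-attack loop; montage notifies enable the HitBox overlap, and a box trace applies damage to the player.
; The construction script randomizes walk speed and skeletal mesh.
; Death plays montage, sound and blood decal, notifies player and spawner, then destroys the actor after a delay.
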(event `self.ReceiveBeginPlay`
  (`parent.ReceiveBeginPlay`)
  (`self.Roaming`))

(event `Roaming`
  (if (`|EnumEquality` (`self.States`) "NewEnumerator0")
    (bind _randomlocation (`NavigationSystemV1.K2_GetRandomLocationInNavigableRadius` (`self.K2_GetActorLocation`) 1500.0 null null))
    (`|AIMoveTo` (`AIBlueprintHelperLibrary.GetAIController` self) null _randomlocation null
      (:`OnSuccess`
        (`KismetSystemLibrary.Delay` 2.0)
        (`self.Roaming`))
      (:`OnFail`
        (`self.Roaming`)))))

(event `self.PawnSensing.OnSeePawn`
  (params (Pawn :type "Pawn Object Reference"))
  (if (and (`self.ActorHasTag` Pawn "Player") (not (`self.IsDie`)))
    (set `self.target` Pawn)
    (`self.MoveToTarget`)))

(event `MoveToTarget`
  (bind _target (`self.target`))
  (if (not (or (`self.IsDie`) (`|EnumEquality` (`self.States`) "NewEnumerator1")))
    (`/Engine/EditorBlueprintResources/StandardMacros.IsValid` _target
      (:`Is Valid`
        (set `self.States` "NewEnumerator2")
        (`|AIMoveTo` (`AIBlueprintHelperLibrary.GetAIController` self) null (0.0 0.0 0.0) _target 70.0
          (:`OnSuccess`
            (`self.Attack`))
          (:`OnFail`
            (`self.MoveToTarget`)))))))

(event `Attack`
  (if (`|EnumEquality` (`self.States`) "NewEnumerator2")
    (set `self.States` "NewEnumerator1")
    (`|PlayMontage` (`self.Mesh`) "/Game/MurratProj/Animation/Anim_Sample/ZonbieMove/zombie_attack_Montage.zombie_attack_Montage" 1.0 0.0 "PunchR"
      (:`OnCompleted`
        (set `self.States` "NewEnumerator2" :!label _label)
        (`self.CheckTargetDist`))
      (:`OnInterrupted`
        (goto _label))
      (:`OnNotifyBegin`
        (`PrimitiveComponent.SetCollisionResponseToChannel` (`self.HitBox`) "ECC_Pawn" "ECR_Overlap"))
      (:`OnNotifyEnd`
        (`PrimitiveComponent.SetCollisionResponseToChannel` (`self.HitBox`) "ECC_Pawn" "ECR_Ignore")))))

(event `/Game/MurratProj/Blueprint/Character_BP/Hit_Interface.PawnHit`
  (params (Damage :type "Float (double-precision)"))
  (`|PlayMontage` (`self.Mesh`) "/Game/PolygonCity/Meshes/Characters/Animation/WalkProAnim_Root/Sword_Hit_L_1_Montage.Sword_Hit_L_1_Montage" 1.0 0.0 (select `int` (`KismetMathLibrary.RandomInteger` 4) :`0` "Hit1" :`1` "Hit2" :`2` "Hit3" :`3` "Hit4" :!type "Name")
    (:`then`
      (`GameplayStatics.PlaySoundAtLocation` "/Game/MurratProj/Sound/damage_1_Cue.damage_1_Cue" (`self.K2_GetActorLocation`) (struct) 1.0 1.0 0.0 "/Game/MurratProj/Sound/NewSoundAttenuation.NewSoundAttenuation" null null null))))

(event `self.HitBox.OnComponentBeginOverlap`
  (params (OverlappedComponent :type "PrimitiveComponent Object Reference") (OtherActor :type "Actor Object Reference") (OtherComp :type "PrimitiveComponent Object Reference") (OtherBodyIndex :type Integer) (bFromSweep :type Boolean) (SweepResult :type "HitResult Structure (by ref)"))
  (if (`self.ActorHasTag` OtherActor "player")
    (`KismetSystemLibrary.PrintString` "Hit")
    (`self.HitPlayer` (`BoxComponent.GetScaledBoxExtent` (`self.HitBox`)))))

(event `DestroyDie`
  (`KismetSystemLibrary.Delay` 20.0)
  (`self.K2_DestroyActor`))

(fn `CheckTargetDist`
  (bind _target (`self.target`)
    (:`then`
      (if (> (`self.GetDistanceTo` _target self) 70.0)
        (`self.MoveToTarget`)
        (else
          (`self.Attack`))))
    (:`else`)))

(fn `Dying`
  (bind _returnvalue (`KismetMathLibrary.RandomFloatInRange` 0.0 360.0))
  (`parent.Dying`)
  (`AnimInstance.Montage_Play` (`SkeletalMeshComponent.GetAnimInstance` (`self.Mesh`)) "/Game/MurratProj/Animation/Anim_Sample/ZonbieMove/zombie_death_Montage.zombie_death_Montage" 1.0 "MontageLength" 0.0 true)
  (`GameplayStatics.PlaySoundAtLocation` "/Game/MurratProj/Sound/ZombieDie.ZombieDie" (`self.K2_GetActorLocation`) (struct) 1.0 1.0 0.0 null null null null)
  (`MovementComponent.StopMovementImmediately` (`self.CharacterMovement`))
  (`Controller.StopMovement` (`AIBlueprintHelperLibrary.GetAIController` self))
  (`PrimitiveComponent.SetCollisionEnabled` (`self.CapsuleComponent`) "NoCollision")
  (message `/Game/MurratProj/Blueprint/Character_BP/Hit_Interface.NotifyKill` (`GameplayStatics.GetPlayerCharacter` 0) (`GameplayStatics.GetObjectClass` self) (`self.EnnemiValue`))
  (message `/Game/MurratProj/Blueprint/Character_BP/MissionInterface.CheckKill` (`self.SpawnerRef`))
  (`GameplayStatics.SpawnDecalAtLocation` "/Game/MurratProj/Textures/Environment/Material/M_DecalBlood01.M_DecalBlood01" (32.0 128.0 128.0) (- (`self.K2_GetActorLocation`) (`KismetMathLibrary.MakeVector` 0.0 0.0 (`.OutHalfHeight` (`CapsuleComponent.GetScaledCapsuleSize` (`self.CapsuleComponent`))))) (`KismetMathLibrary.MakeRotator` _returnvalue -90.0 _returnvalue))
  (`Controller.UnPossess` (`self.GetController`))
  (`self.DestroyDie`))

(fn `HitPlayer`
  (params (BoxExtend :type "Vector Structure"))
  (bind _returnvalue (`SceneComponent.K2_GetComponentLocation` (`self.HitBox`)))
  (bind _outhits (`KismetSystemLibrary.BoxTraceMultiForObjects` _returnvalue (+ _returnvalue (5.0 0.0 0.0)) BoxExtend (struct) (`|MakeArray` "ObjectTypeQuery3" :!type "EObjectTypeQuery Enum") false (`|MakeArray` self :!type "Actor Object Reference")))
  (for _array_element _outhits
    (bind (_bblockinghit _binitialoverlap _time _distance _location _impactpoint _normal _impactnormal _physmat _hitactor) (`GameplayStatics.BreakHitResult` _array_element))
    (`/Engine/EditorBlueprintResources/StandardMacros.IsValid` _hitactor
      (:`Is Valid`
        (if (`self.ActorHasTag` _hitactor "player")
          (`GameplayStatics.ApplyDamage` _hitactor 10.0)
          (`GameplayStatics.PlaySound2D` "/Game/MurratProj/Sound/damage_1_Cue.damage_1_Cue" 1.0 1.0 0.0 null null))))))

(fn `MoveTo`)

(fn `UserConstructionScript`
  (`parent.UserConstructionScript`)
  (set `CharacterMovementComponent.MaxWalkSpeed` (`KismetMathLibrary.SelectFloat` 75.0 225.0 (`KismetMathLibrary.RandomBool`)) (`self.CharacterMovement`))
  (set `SkeletalMeshComponent.SkeletalMeshAsset` (select `int` (`KismetMathLibrary.RandomInteger` 7) :`0` "/Game/PolygonCityChar/Characters/SK_Character_FastFoodGuy.SK_Character_FastFoodGuy" :`1` "/Game/PolygonCityChar/Characters/SK_Character_HipsterGirl.SK_Character_HipsterGirl" :`2` "/Game/PolygonCityChar/Characters/SK_Character_Hotdog.SK_Character_Hotdog" :`3` "/Game/PolygonCityChar/Characters/SK_Character_PunkGuy.SK_Character_PunkGuy" :`4` "/Game/PolygonCityChar/Characters/SK_Character_ShopKeeper.SK_Character_ShopKeeper" :`5` "/Game/PolygonCityChar/Characters/SK_Character_SummerGirl.SK_Character_SummerGirl" :`6` "/Game/PolygonCityChar/Characters/SK_Character_Tourist.SK_Character_Tourist" :!type "SkeletalMesh Object Reference") (`self.Mesh`)))